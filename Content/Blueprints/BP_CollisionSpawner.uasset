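; BP_CollisionSpawner scatters BP_Collision actors over a landscape within its SpawnVolume box.
; Scatter destroys the previously spawned actors, then runs Quantity-based line traces against WorldStatic objects, using random box points offset far below and above.
; Hits on the referenced Landscape spawn an actor at the impact point, oriented from the rotated surface normal, and track it in EarlierCollision for the next cleanup.
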(event `Scatter`
  (bind _earliercollision (`self.EarlierCollision`))
  (bind _returnvalue (`KismetMathLibrary.RandomPointInBoundingBox` (`self.K2_GetActorLocation`) (`BoxComponent.GetScaledBoxExtent` (`self.SpawnVolume`))))
  (for _array_element _earliercollision
    (`self.K2_DestroyActor` _array_element))
  (`KismetArrayLibrary.Array_Resize` _earliercollision)
  (`KismetArrayLibrary.Array_Clear` _earliercollision)
  (for _ (range (+ (`self.Quantity`) 1))
    (bind _outhit (`KismetSystemLibrary.LineTraceSingleForObjects` :`Start` (- _returnvalue (0.0 0.0 2000.0)) :`End` (+ _returnvalue (0.0 0.0 2000.0)) :`ObjectTypes` (`|MakeArray` "ObjectTypeQuery1" :!type "EObjectTypeQuery Enum") :`DrawDebugType` "ForOneFrame"))
    (if (== (`self.Landscape`) (`.HitActor` (`GameplayStatics.BreakHitResult` _outhit)))
      (bind _returnvalue_2 (`|SpawnActorFromClass` "/Game/Blueprints/BP_Collision.BP_Collision_C" (`KismetMathLibrary.MakeTransform` (`.Location` (`GameplayStatics.BreakHitResult` _outhit)) (`KismetMathLibrary.Conv_VectorToRotator` (`KismetMathLibrary.GreaterGreater_VectorRotator` (`.Normal` (`GameplayStatics.BreakHitResult` _outhit)) (struct :`Pitch` 90.0)))) "Undefined" "OverrideRootScale" null null))
      (`KismetArrayLibrary.Array_Add` (`self.EarlierCollision`) _returnvalue_2))))

(fn `UserConstructionScript`)