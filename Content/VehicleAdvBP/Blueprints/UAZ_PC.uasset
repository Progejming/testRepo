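; UAZ_PC is a player controller that lets the player sculpt voxel terrain with the mouse.
; ProjectionEditEvent checks local control and left-button hold time, then sends the cursor ray to ServerProjectionEdit, with held Left Ctrl selecting add mode.
; ServerProjectionEdit finds the voxel world along that ray and applies a projection edit along the hit normal.
; The local GetVoxelWorld graph holds only unconnected cursor-trace debug logic.
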(event `ServerProjectionEdit`
  (params (`World Position` :type "Vector Structure") (`World Direction` :type "Vector Structure") (Radius :type "Float (double-precision)") (bAdd :type Boolean))
  (bind _bdebug (`self.bDebug`))
  ;[1 1 1] Server projection edit
  (bind (_world _hitposition _hitnormal) (`VoxelTools.GetVoxelWorld` `World Position` `World Direction` (`self.MaxEditDistance`) self)
    (:`Success`
      (`VoxelTools.SetValueProjection` _world _hitposition _hitnormal Radius 0.1 bAdd (`self.ProjectionEditDistance`) 0.25 true _bdebug _bdebug _bdebug))))

(event `ProjectionEditEvent`
  ;[1 1 1] Projection edit
  (if (`self.IsLocalPlayerController`)
    (if (>= (`self.GetInputKeyTimeDown` "LeftMouseButton") (`self.EditDelay`))
      (bind (_worldposition _worlddirection) (`VoxelTools.GetMouseWorldPositionAndDirection` self)
        (:`Success`
          (`self.ServerProjectionEdit` _worldposition _worlddirection (`self.Radius`) (>= (`self.GetInputKeyTimeDown` "LeftControl") (`self.EditDelay`))))))))

(fn `UserConstructionScript`)